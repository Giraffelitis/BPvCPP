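; Shootable benchmark target in a testing hub, built to compare Blueprint and C++ loop performance.
; On BeginPlay it labels itself with test ID, iteration count and method name; a projectile overlap destroys the projectile and runs a timed test.
; Wall-clock milliseconds and the result are printed.
; The overlap is wired straight to the C++ += test; the TestID switch is disconnected, and IDs from 8 up are unfinished stubs.
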(event `self.SphereComp.OnComponentBeginOverlap`
  (params (OverlappedComponent :type "PrimitiveComponent Object Reference") (OtherActor :type "Actor Object Reference") (OtherComp :type "PrimitiveComponent Object Reference") (OtherBodyIndex :type Integer) (bFromSweep :type Boolean) (SweepResult :type "HitResult Structure (by ref)"))
  (bind _asbp_first_person_projectile (cast `/Game/FirstPerson/Blueprints/BP_FirstPersonProjectile` OtherActor))
  (`self.K2_DestroyActor` _asbp_first_person_projectile)
  (set `self.Result` 0)
  ;[0 0.5669 1] Simple Addition Routes
  (`self.GetStartTime`)
  ;;[1 1 1] TEST ID 1 = CPP +=
  (`self.StartTestIterations` (`self.NumOfIterations`))
  (bind _returnvalue (`self.CalculateIterationTime`))
  (`KismetSystemLibrary.PrintString` _returnvalue true true (struct :`G` 0.66 :`B` 1.0 :`A` 1.0) 30.0))

(event `self.ReceiveBeginPlay`
  (`self.SetTargetsText`))

(fn `CalculateIterationTime`
  (returns (ReturnValue :type String))
  (return (`KismetStringLibrary.Concat_StrStr` (`KismetStringLibrary.Conv_DoubleToString` (`KismetMathLibrary.GetTotalMilliseconds` (- (`KismetMathLibrary.GetTimeOfDay` (`KismetMathLibrary.Now`)) (`self.Timespan`)))) "ms result:" (`KismetStringLibrary.Conv_IntToString` (`self.Result`)))))

(fn `GetStartTime`
  (set `self.Timespan` (`KismetMathLibrary.GetTimeOfDay` (`KismetMathLibrary.Now`))))

(fn `SetTargetsText`
  (set `self.IDText` (`KismetTextLibrary.Conv_IntToText` (`self.TestID`)))
  (set `self.InterationsText` (`KismetTextLibrary.Conv_IntToText` (`self.NumOfIterations`)))
  (switch `int` (`self.TestID`)
    (:`0`
      (set `self.MethodText` "BP +="))
    (:`1`
      (set `self.MethodText` "CPP +="))
    (:`2`
      (set `self.MethodText` "BP CPP +="))
    (:`3`
      (set `self.MethodText` "BP ++"))
    (:`4`
      (set `self.MethodText` "CPP ++"))
    (:`5`
      (set `self.MethodText` "BP CPP ++"))
    (:`6`
      (set `self.MethodText` "BP Branch"))
    (:`7`
      (set `self.MethodText` "CPP Branch"))
    (:`8`
      (set `self.MethodText` ""))
    (:`9`
      (set `self.MethodText` ""))
    (:`10`
      (set `self.MethodText` ""))
    (:`11`
      (set `self.MethodText` ""))
    (:`12`
      (set `self.MethodText` ""))
    (:`13`
      (set `self.MethodText` ""))
    (:`14`
      (set `self.MethodText` ""))
    (:`15`
      (set `self.MethodText` ""))
    (:`16`
      (set `self.MethodText` ""))
    (:`17`
      (set `self.MethodText` ""))
    (:`18`
      (set `self.MethodText` ""))
    (:`19`
      (set `self.MethodText` ""))
    (:`20`
      (set `self.MethodText` ""))
    (:`21`
      (set `self.MethodText` ""))
    (:`22`
      (set `self.MethodText` ""))
    (:`23`
      (set `self.MethodText` "")))
  (`TextRenderComponent.K2_SetText` (`self.ID Text`) (`self.IDText`))
  (`TextRenderComponent.K2_SetText` (`self.Iterations Text`) (`self.InterationsText`))
  (`TextRenderComponent.K2_SetText` (`self.Method Text`) (`self.MethodText`)))

(fn `UserConstructionScript`)